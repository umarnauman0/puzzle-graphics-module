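; BP_ElementBlock is a rotatable puzzle block with a glowing rune that reports to a parent tower.
; RotateBlock cycles through four quarter-turn yaw positions, then EvaluateAlignment compares the index to the correct one, locking the block on a match.
; A dynamic material shows green or red rune feedback, and each evaluation asks the tower to check if solved.
; ResetBlock clears state, unlocks the block and restores a purple rune.
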(event Custom|RotateBlock
  (bind _blockmesh (Variables|Default|GetBlockMesh))
  (if (not (Variables|Default|GetbLocked))
    (if (Variables|Default|GetbIsAligned)
      (Development|PrintString "Already Solved")
      (else
        (bind _result (Math|Integer|IncrementInt (Variables|Default|GetCurrentIndex))
          (:%20%20
            (bind _output_get (Variables|Default|SetCurrentIndex (Math|Integer|%(Integer) _result 4)))
            (Components|MoveComponentTo _blockmesh (Variables|/Script/Engine.SceneComponent|GetRelativeLocation _blockmesh) (Math|Rotator|MakeRotator 0.0 0.0 (.yaw (Math|Rotator|MakeRotator 0.0 0.0 (Math|Conversions|ToFloat(Integer) (* _output_get 90))))) false false 1.0 false)
            (CallFunction|EvaluateAlignment)))))))

(event Custom|EvaluateAlignment
  (bind _matinstance (Variables|Default|GetMatInstance))
  (bind _matinstance_2 (Variables|Default|GetMatInstance))
  (bind _parenttowerref (Variables|Default|GetParentTowerRef))
  ;[0.15 0.15 0.15 0.5] Evaluate Correct Block Alignment
  (if (== (Variables|Default|GetCurrentIndex) (Variables|Default|GetCorrectIndex))
    (Variables|Default|SetbIsAligned true)
    (Variables|Default|SetbLocked true)
    (Rendering|Material|SetScalarParameterValue _matinstance "Glow" 1e+01 :!class /Script/Engine.MaterialInstanceDynamic)
    (Rendering|Material|SetVectorParameterValue _matinstance_2 "RuneColour" "(R=0.044169,G=1.000000,B=0.000000,A=1.000000)" :!class /Script/Engine.MaterialInstanceDynamic)
    (Development|PrintString "Correct")
    (else
      (Variables|Default|SetbIsAligned false)
      (Rendering|Material|SetScalarParameterValue _matinstance "Glow" 4.0 :!class /Script/Engine.MaterialInstanceDynamic)
      (Rendering|Material|SetVectorParameterValue _matinstance_2 "RuneColour" "(R=1.000000,G=0.000000,B=0.000000,A=1.000000)" :!class /Script/Engine.MaterialInstanceDynamic)
      (Development|PrintString "Not Correct")))
  (if (Utilities|IsValid _parenttowerref)
    (Default|CheckSolved _parenttowerref)))

(event Custom|ResetBlock
  (bind _blockmesh (Variables|Default|GetBlockMesh))
  (Variables|Default|SetCurrentIndex 0)
  (Variables|Default|SetbIsAligned false)
  (Variables|Default|SetbLocked false)
  (Components|MoveComponentTo _blockmesh (Variables|/Script/Engine.SceneComponent|GetRelativeLocation _blockmesh) (Math|Rotator|MakeRotator 0.0 0.0 0.0) false false 1.0 false)
  (Rendering|Material|SetVectorParameterValue (Variables|Default|GetMatInstance) "RuneColour" "(R=0.331635,G=0.000000,B=1.000000,A=1.000000)" :!class /Script/Engine.MaterialInstanceDynamic))

(event EventBeginPlay
  (bind _returnvalue (Rendering|Material|CreateDynamicMaterialInstance (Variables|Default|GetBlockMesh) 0 (Variables|Default|GetMatInstance) "None" :!class /Script/Engine.PrimitiveComponent))
  (bind _output_get (Variables|Default|SetMatInstance _returnvalue))
  (Rendering|Material|SetScalarParameterValue _output_get "Glow" 2.0 :!class /Script/Engine.MaterialInstanceDynamic))

(event Collision|EventActorBeginOverlap
  (params (OtherActor :type Actor%20Object%20Reference)))

(event EventTick
  (params (DeltaSeconds :type Float%20%28single-precision%29)))

(fn ConstructionScript)