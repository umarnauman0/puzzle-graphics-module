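; BP_Tower is a puzzle actor that is solved when all of its Blocks are aligned.
; CheckSolved, gated by CanCheck, scans the blocks and calls ResetTower on the first misaligned one, which resets every block and re-enables checking after a delay.
; OnTowerSolvedLogic sets IsSolved, disables checking and calls OnTowerSolved.
; As wired, that solved logic also runs after a failed check breaks the loop.
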(event Custom|CheckSolved
  (if (Variables|Default|GetbCanCheck)
    (bind _array_element (Utilities|Array|ForEachLoopwithBreak (Variables|Default|GetBlocks) :!label _label)
      (:LoopBody
        (bind _output_get (Variables|Default|SetCurrentBlock _array_element)) ; Array Element
        (if (not (Variables|/Game/_Puzzle/Blueprints/BP_ElementBlock.BP_ElementBlock_C|GetbIsAligned _output_get))
          (CallFunction|ResetTower)
          (goto _label Break)))
      (:Completed
        (CallFunction|OnTowerSolvedLogic)))))

(event Custom|ResetTower
  (Development|PrintString "Incorrect combination!")
  (for _array_element (Variables|Default|GetBlocks)
    (bind _output_get (Variables|Default|SetCurrentBlock _array_element))
    (Default|ResetBlock _output_get)
    (Utilities|FlowControl|Delay 2.0)
    (Variables|Default|SetbCanCheck true)))

(event Custom|OnTowerSolvedLogic
  (Variables|Default|SetbIsSolved true)
  (Variables|Default|SetbCanCheck false)
  (Development|PrintString "Tower Solved!")
  (Default|CallOnTowerSolved))

(event EventBeginPlay)

(event Collision|EventActorBeginOverlap
  (params (OtherActor :type Actor%20Object%20Reference)))

(event EventTick
  (params (DeltaSeconds :type Float%20%28single-precision%29)))

(fn ConstructionScript)